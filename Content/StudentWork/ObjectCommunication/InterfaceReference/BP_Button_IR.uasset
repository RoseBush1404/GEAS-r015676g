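; BP_Button_IR is an interactable button that toggles an array of target objects on and off through interface messages.
; Its trigger volume binds an event to the overlapping character's player-interact dispatcher on entry and unbinds it on exit, getting that character through an interface message.
; TriggerButton flip-flops between states, messaging each target and switching the button light between green and red via a dynamic material created in the construction script.
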(event `self.Trigger collision.OnComponentBeginOverlap`
  (params (OverlappedComponent :type "PrimitiveComponent Object Reference") (OtherActor :type "Actor Object Reference") (OtherComp :type "PrimitiveComponent Object Reference") (OtherBodyIndex :type Integer) (bFromSweep :type Boolean) (SweepResult :type "HitResult Structure (by ref)"))
  ;[1 1 1] Bind event when player enters area, and unbind when they leave
  (bind _basecharacterref (message `/Game/StudentWork/InterFaces/iCharacterRefSystem.CharacterSelfBaseCharacterRef` OtherActor))
  (add `/Game/StudentWork/Characters/BaseCharacter.PlayerInteractDispatcher` _basecharacterref (`|CreateDelegate` :!event `TriggerButton`)))

(event `self.Trigger collision.OnComponentEndOverlap`
  (params (OverlappedComponent :type "PrimitiveComponent Object Reference") (OtherActor :type "Actor Object Reference") (OtherComp :type "PrimitiveComponent Object Reference") (OtherBodyIndex :type Integer))
  ;[1 1 1] Bind event when player enters area, and unbind when they leave
  (bind _basecharacterref (message `/Game/StudentWork/InterFaces/iCharacterRefSystem.CharacterSelfBaseCharacterRef` OtherActor))
  (remove `/Game/StudentWork/Characters/BaseCharacter.PlayerInteractDispatcher` _basecharacterref (`|CreateDelegate` :!event `TriggerButton`)))

(event `TriggerButton`
  (bind _button_light_material (`self.Button light material`))
  (bind _targetobject (`self.TargetObject`))
  ;[1 1 1] Toggle on and off
  (`/Engine/EditorBlueprintResources/StandardMacros.FlipFlop`
    (:`A`
      (`MaterialInstanceDynamic.SetScalarParameterValue` _button_light_material "State" 1.0) ; Change a scalar value in the button material that turns it green
      (for _array_element _targetobject
        (message `/Game/StudentWork/ObjectCommunication/InterfaceReference/iBulbSystem.ToggleOn` _array_element)))
    (:`B`
      (`MaterialInstanceDynamic.SetScalarParameterValue` _button_light_material "State" 0.0) ; Change a scalar value in the button material that turns it back to red
      (for _array_element_2 _targetobject
        (message `/Game/StudentWork/ObjectCommunication/InterfaceReference/iBulbSystem.ToggleOff` _array_element_2)))))

(fn `UserConstructionScript`
  (bind _returnvalue (`PrimitiveComponent.CreateDynamicMaterialInstance` (`self.ButtonMesh`) 2 null))
  (set `self.Button light material` _returnvalue) ; Save a reference to the Dynamic Material Instance for use in the event graph
)